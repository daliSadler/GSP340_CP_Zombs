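; Interactable switch, built on a parent interaction Blueprint, that toggles three point lights.
; Interact calls the parent, flips Active, nudges the switch mesh along local or relative X and sets the prompt to "Turn Off" or "Turn On".
; The lights toggle visibility rather than following Active, and only when the interaction widget is valid.
; CallActivate and CallDeactivate nodes are left unconnected.
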(event EventInteract
  (params (Character :type First%20Person%20Character%20Object%20Reference))
  (bind _interactmesh (Variables|Default|GetInteractMesh))
  (bind _pointlight (Variables|Default|GetPointLight))
  ;[1 1 1] Interact (Switch)
  (|CallParentFunction Character)
  (if (not (Variables|Default|GetbActive))
    (Variables|Default|SetbActive true)
    (Transformation|AddRelativeLocation _interactmesh "3.000000,0.000000, 0" false false)
    (bind _interactionuiwidget (Variables|Default|GetInteractionUIWidget)
      (:then
        (Default|SetInteractDescription _interactionuiwidget "Turn Off")
        (Rendering|ToggleVisibility _pointlight false))
      (:else))
    (else
      (Variables|Default|SetbActive false)
      (Transformation|AddRelativeLocation _interactmesh "-3.000000,0.000000, 0" false false)
      (bind _interactionuiwidget_2 (Variables|Default|GetInteractionUIWidget)
        (:then
          (Default|SetInteractDescription _interactionuiwidget_2 "Turn On")
          (Rendering|ToggleVisibility _pointlight false))
        (:else)))))

(fn ConstructionScript
  (|CallParentFunction))